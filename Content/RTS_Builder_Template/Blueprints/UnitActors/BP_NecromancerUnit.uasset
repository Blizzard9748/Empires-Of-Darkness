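; BP_NecromancerUnit is an RTS necromancer unit whose first ability button casts Raise Dead.
; The ability spawns a BP_ZombieUnit at the Spawner transform, has a newly spawned BP_UnitController possess it, and attaches detection by spawning a BP_DetectionRange told to follow the zombie.
; The second button is empty, and a timed attack-speed buff is left unconnected.
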(event `self.Button 1 Clicked`
  (bind _returnvalue (`SceneComponent.K2_GetComponentToWorld` (`self.Spawner`)))
  ;[1 1 1] Raise Dead Ability
  (bind _returnvalue_2 (`|SpawnActorFromClass` "/Game/RTS_Builder_Template/Blueprints/UnitActors/BP_UnitController.BP_UnitController_C" _returnvalue "AlwaysSpawn" "MultiplyWithRoot" null null))
  (bind _returnvalue_3 (`|SpawnActorFromClass` "/Game/RTS_Builder_Template/Blueprints/UnitActors/BP_ZombieUnit.BP_ZombieUnit_C" _returnvalue "AlwaysSpawn" "SelectDefaultAtRuntime" null "NewEnumerator4" null))
  (`Controller.Possess` _returnvalue_2 _returnvalue_3)
  (bind _returnvalue_4 (`|SpawnActorFromClass` "/Game/RTS_Builder_Template/Blueprints/Others/BP_DetectionRange.BP_DetectionRange_C" (`KismetMathLibrary.MakeTransform` (0.0 0.0 0.0)) "Undefined" "OverrideRootScale" null null))
  (`/Game/RTS_Builder_Template/Blueprints/Others/BP_DetectionRange.On Spawned` _returnvalue_4 _returnvalue_3 0.0))

(event `self.Button 2 Clicked`)

(fn `Trace All Rotation_0_0`
  (returns (Location :type "Vector Structure"))
  (return (`self.K2_GetActorLocation`)))

(fn `UserConstructionScript`
  (`parent.UserConstructionScript`))