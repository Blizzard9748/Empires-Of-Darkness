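; BP_Ranger_Base is a base ranged AI character in the RTS builder template, with a placeholder attack.
; Attack waits briefly, signals attack end and prints debug text, with no damage or projectile logic.
; GetPatrolRoute exposes the patrol route, and SetMovementSpeed maps idle, walking and sprinting states to walk speed.
; BeginPlay and ChasePlayer are empty; the builder-unit chase-and-attack loop and montage playback are disconnected.
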(event `self.ReceiveBeginPlay`)

(event `ChasePlayer`)

(event `Attack`
  (`KismetSystemLibrary.Delay` 0.5)
  (`self.OnAttackEnd`)
  (`KismetSystemLibrary.PrintText` "Attack"))

(fn `GetPatrolRoute`
  (returns (PatrolRoute :type "/Game/RTS_Builder_Template/Blueprints/RangedAI/RangedAI_Tree/BP_Patrol_Route Object Reference"))
  (return (`self.PatrolRoute`)))

(fn `SetMovementSpeed`
  (params (Speed :type "/Game/RTS_Builder_Template/Blueprints/RangedAI/RangedAI_Tree/Enums/E_MovementSpeed Enum" :default "NewEnumerator0"))
  (returns (SpeedValue :type "Float (double-precision)"))
  (set `CharacterMovementComponent.MaxWalkSpeed` (select `/Game/RTS_Builder_Template/Blueprints/RangedAI/RangedAI_Tree/Enums/E_MovementSpeed` Speed :`NewEnumerator1` 300.0 :`NewEnumerator2` 500.0 :!type "Float (single-precision)") (`self.CharacterMovement`))
  (return 0.0))

(fn `UserConstructionScript`)