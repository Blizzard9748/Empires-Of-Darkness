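; BP_ZombieHeavySpawner is a recruitment building in the RTS template, named for heavy zombie units.
; Its first button recruits the RecruitmentUnit, and its second buys capped damage and attack speed upgrades for that unit at a food cost.
; SetHUDVisibilitys has the RTS pawn display the shared Barracks HUD.
; The recruit and upgrade logic is called rather than defined here, and BeginPlay and Tick are disabled stubs.
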(event `self.Button 1 Clicked`
  (`self.Recruit Unit` (`self.Recruitment Unit`)))

(event `self.Button 2 Clicked`
  (`self.Upgrade Units` 3 0.0 0 (`self.Recruitment Unit`) 2.0 0.25 200))

(event `self.Set HUD Visibilitys`
  (`/Game/RTS_Builder_Template/Blueprints/Player/BP_RTSPawn.Set HUD Visibilitys` (`self.RTS Pawn`) "Hidden" "Visible" "Hidden" "Hidden" "Hidden" "Hidden" "Hidden" "Visible" "Hidden" "Hidden"))

(fn `UserConstructionScript`
  (`parent.UserConstructionScript`))