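; BP_ZombieHomebase is the zombie homebase building in the RTS builder template, used to recruit zombie-side units.
; Its two button events call the inherited RecruitUnit to produce a BP_ZombieBuilder or a BP_NecromancerUnit.
; Its SetHUDVisibilitys event has the RTS pawn show the Barracks HUD rather than a HUD specific to this building.
; BeginPlay, Tick and the construction script add nothing beyond the parent class.
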(event `self.Button 1 Clicked`
  (`self.Recruit Unit` "/Game/RTS_Builder_Template/Blueprints/UnitActors/BP_ZombieBuilder.BP_ZombieBuilder_C"))

(event `self.Button 2 Clicked`
  (`self.Recruit Unit` "/Game/RTS_Builder_Template/Blueprints/UnitActors/BP_NecromancerUnit.BP_NecromancerUnit_C"))

(event `self.Set HUD Visibilitys`
  (`/Game/RTS_Builder_Template/Blueprints/Player/BP_RTSPawn.Set HUD Visibilitys` (`self.RTS Pawn`) "Hidden" "Visible" "Hidden" "Hidden" "Hidden" "Hidden" "Hidden" "Visible" "Hidden" "Hidden"))

(fn `UserConstructionScript`
  (`parent.UserConstructionScript`))